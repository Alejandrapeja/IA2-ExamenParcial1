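; BP_ANode is an A* graph node that shows its name and uses arrow materials to mark start, goal, visited and final path.
; The goal node assigns heuristics by recursively growing its box and stamping the ring level on overlapping, still-unset nodes, up to a fixed depth.
; Each node randomizes its risk cost unless set manually, and exposes setters for total and accumulated costs.
; Runtime click selection of start and goal is disconnected.
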(event `self.ReceiveBeginPlay`
  ;[1 1 1] Asignar materiales y nombre al display
  (`self.StartVisual`)
  (`self.GoalViasual`)
  (`TextRenderComponent.K2_SetText` (`self.TextRender`) (`KismetTextLibrary.Conv_StringToText` (`KismetSystemLibrary.GetDisplayName` self)))
  (`self.Cost`))

(event `PassedVisual`
  ;[1 1 1] Cambio de materiales si se analizo y si forma parte del camino final
  (`PrimitiveComponent.SetMaterial` (`self.Arrow`) 0 "/Game/AI/Materials/MI_ArrowVisited.MI_ArrowVisited"))

(event `PathVisual`
  ;[1 1 1] Cambio de materiales si se analizo y si forma parte del camino final
  (`PrimitiveComponent.SetMaterial` (`self.Arrow`) 0 "/Game/AI/Materials/MI_ArrowPath.MI_ArrowPath"))

(event `StartVisual`
  ;[0.2544 0.5052 0.2439] Si nodo es START
  (if (`self.Start`)
    (`PrimitiveComponent.SetMaterial` (`self.Arrow`) 0 "/Game/AI/Materials/MI_ArrowStart.MI_ArrowStart")))

(event `GoalViasual`
  ;[0.6094 0.3039 0.2917] Si nodo es GOAL
  (if (`self.Goal`)
    (`PrimitiveComponent.SetMaterial` (`self.Arrow`) 0 "/Game/AI/Materials/MI_ArroeGoal.MI_ArroeGoal")
    (`BoxComponent.SetBoxExtent` (`self.Box`) (375.0 375.0 30.0) true)
    (`self.CalculoHeuristica`)))

(event `CalculoHeuristica`
  (bind _box (`self.Box`))
  (bind _nivelesh (`self.NivelesH`))
  ;[1 1 1] Aestrella
  ;;[1 1 1] Asignar costos Heulistica
  (if (<= _nivelesh 8)
    (`/Engine/EditorBlueprintResources/StandardMacros.IncrementInt` _nivelesh
      (:`  `
        (for _array_element (`PrimitiveComponent.GetOverlappingActors` (`self.Box`) "BP_ANode_C")
          (bind _asbp_anode (cast `/Game/AI/Actors/BP_ANode` _array_element)
            (:`then`
              (if (== 0 (`/Game/AI/Actors/BP_ANode.Heuristica` _asbp_anode))
                (if (not (`/Game/AI/Actors/BP_ANode.Goal` _asbp_anode))
                  (set `/Game/AI/Actors/BP_ANode.Heuristica` (`self.NivelesH`) _asbp_anode))
                (else
                  (`KismetSystemLibrary.PrintString` "Set H Detected" true true (struct :`R` 0.861831 :`G` 1.0 :`A` 1.0)))))
            (:`CastFailed`
              (`KismetSystemLibrary.PrintString` "Overlaping actor =! ANode" true true (struct :`R` 1.0 :`B` 0.027472 :`A` 1.0) 10.0))))
        (`BoxComponent.SetBoxExtent` _box (+ (`BoxComponent.BoxExtent` _box) (`KismetMathLibrary.MakeVector` 250.0 250.0)) true)
        (`self.CalculoHeuristica`)))
    (else
      (`KismetSystemLibrary.PrintString` "Finished Calculating Heustics" true true (struct :`G` 1.0 :`B` 0.324347 :`A` 1.0) 5.0))))

(event `Cost`
  ;[1 1 1] Aestrella
  ;;[1 1 1] Costo Aleatoreo?
  (if (not (`self.CostoRiesgosManual?`))
    (set `self.CostoRiesgos` (`KismetMathLibrary.RandomIntegerInRange` 0 3))))

(event `CalculateTotal`
  (params (CostoTotal :type Integer))
  ;[1 1 1] Aestrella
  ;;[1 0.8973 0.3638] Calcular costo total y acumulativo
  (set `self.CostoTotal` CostoTotal))

(event `CalculateAcumulative`
  (params (CostoAcumulativoG :type Integer))
  ;[1 1 1] Aestrella
  ;;[1 0.8973 0.3638] Calcular costo total y acumulativo
  (set `self.CostoAcumulativoG` CostoAcumulativoG))

(event `self.Arrow.OnClicked`
  (params (TouchedComponent :type "PrimitiveComponent Object Reference") (ButtonPressed :type "Key Structure"))
  ;[0.2969 0.2969 0.2969] Intento de cambiar en runtime
)

(fn `UserConstructionScript`)